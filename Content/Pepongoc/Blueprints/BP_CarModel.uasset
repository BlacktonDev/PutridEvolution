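; BP_CarModel handles a player's input in the lobby, mainly toggling ready state and opening the pause menu.
; On BeginPlay it adds the car-selection mapping context and caches the GS_BaseSetup game state and LobbyHUD.
; IA_Select flips readiness through ServerIsReady, which reports it to the game state's PlayerOnLobby.
; Escape shows WB_PauseMenu with UI-only input, while left/right inputs are empty and player-list widget code is disconnected.
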(event `self.ReceiveBeginPlay`
  (`EnhancedInputSubsystemInterface.AddMappingContext` (pcsubsystem `EnhancedInputLocalPlayerSubsystem` (`GameplayStatics.GetPlayerControllerFromID` 0)) "/Game/Pepongoc/Blueprints/Inputs/IMC_SelectCar.IMC_SelectCar" 0 (struct))
  (bind _asgs_base_setup (cast `/Game/Pepongoc/Blueprints/GameModes/GS_BaseSetup` (`GameplayStatics.GetGameState`)))
  (set `self.PlayerGameState` _asgs_base_setup)
  (bind _aslobby_hud (cast `/Game/Pepongoc/Blueprints/GameModes/Lobby/LobbyHUD` (`PlayerController.GetHUD` (`GameplayStatics.GetPlayerController` 0))))
  (set `self.As Lobby HUD` _aslobby_hud))

(event `Ready`
  ;[1 1 1] no se que hace pero funciona
  (`self.Is Ready` false))

(event `EnhancedInput|/Game/Pepongoc/Blueprints/Inputs/IA/IA_Select`
  (params (ActionValue :type Boolean) (ElapsedSeconds :type "Float (double-precision)") (TriggeredSeconds :type "Float (double-precision)") (InputAction :type "InputAction Object Reference" :default "/Game/Pepongoc/Blueprints/Inputs/IA/IA_Select.IA_Select"))
  (bind _isplayerready (`self.IsPlayerReady`))
  (:`Started`
    (`/Engine/EditorBlueprintResources/StandardMacros.FlipFlop`
      (:`A`
        (set `self.IsPlayerReady` true))
      (:`B`
        (set `self.IsPlayerReady` false)))
    ;[1 1 1] Quien es cliente y quien servidor
    (if (`self.HasAuthority`)
      (`self.Server Is Ready` _isplayerready)
      (else
        (`self.Server Is Ready` _isplayerready)))))

(event `Server Is Ready`
  (params (NewParam :type Boolean))
  ;[1 1 1] no se que hace pero funciona
  (bind _output_get (set `self.IsPlayerReady` NewParam))
  (`self.Is Ready` _output_get))

(event `Is Ready`
  (params (IsReady :type Boolean))
  ;[1 1 1] no se que hace pero funciona
  (`/Game/Pepongoc/Blueprints/GameModes/GS_BaseSetup.Player On Lobby` (`self.PlayerGameState`) IsReady))

(event `self.ReceiveTick`
  (params (DeltaSeconds :type "Float (single-precision)")))

(event `EnhancedInput|/Game/Pepongoc/Blueprints/Inputs/IA/IA_Left`
  (params (ActionValue :type Boolean) (ElapsedSeconds :type "Float (double-precision)") (TriggeredSeconds :type "Float (double-precision)") (InputAction :type "InputAction Object Reference" :default "/Game/Pepongoc/Blueprints/Inputs/IA/IA_Left.IA_Left")))

(event `EnhancedInput|/Game/Pepongoc/Blueprints/Inputs/IA/IA_Right`
  (params (ActionValue :type Boolean) (ElapsedSeconds :type "Float (double-precision)") (TriggeredSeconds :type "Float (double-precision)") (InputAction :type "InputAction Object Reference" :default "/Game/Pepongoc/Blueprints/Inputs/IA/IA_Right.IA_Right")))

(event `Key|Escape`
  (params (Key :type "Key Structure"))
  (bind _returnvalue (`GameplayStatics.GetPlayerController` 0))
  (:`Pressed`
    (bind _returnvalue_2 (`|CreateWidget` "/Game/Pepongoc/Blueprints/UI/PauseMenu/WB_PauseMenu.WB_PauseMenu_C"))
    (`UserWidget.AddToViewport` _returnvalue_2 0)
    (`WidgetBlueprintLibrary.SetInputMode_UIOnlyEx` _returnvalue _returnvalue_2)
    (set `PlayerController.bShowMouseCursor` true _returnvalue)))

(event `Key|Tab`
  (params (Key :type "Key Structure")))

(fn `UserConstructionScript`)