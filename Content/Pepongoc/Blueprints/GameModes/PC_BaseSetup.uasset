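; Lobby player controller that shows the player list and requests a player spawn when play begins.
; BeginPlay adds the WB_PlayerList widget with game-and-UI input and a visible cursor, then the local controller calls SR_SpawnPlayer.
; That event passes the controller to BP_LobbyGame's SpawnPlayer, with debug prints.
; A kick event opens the main menu and destroys the session.
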(event `self.ReceiveBeginPlay`
  ;[1 1 1] Show player List on viewport
  (bind _returnvalue (`|CreateWidget` "/Game/Pepongoc/Blueprints/UI/PlayerList/WB_PlayerList.WB_PlayerList_C" self))
  (`UserWidget.AddToViewport` _returnvalue 0)
  (`WidgetBlueprintLibrary.SetInputMode_GameAndUIEx` self _returnvalue)
  (set `self.bShowMouseCursor` true)
  ;[1 1 1] Spawn Player
  (if (`self.IsLocalPlayerController`)
    (`self.SR_SpawnPlayer`)))

(event `OC_KickPlayer`
  ;[1 1 1] On Kcicked player
  (`GameplayStatics.OpenLevelBySoftObjectPtr` "/Game/Levels/MainMenu.MainMenu")
  (`DestroySessionCallbackProxy.DestroySession` (`GameplayStatics.GetPlayerController` 0)))

(event `SR_SpawnPlayer`
  (bind _asbp_lobby_game (cast `/Game/Pepongoc/Blueprints/GameModes/Lobby/BP_LobbyGame` (`GameplayStatics.GetGameMode`))
    (:`then`
      (`/Game/Pepongoc/Blueprints/GameModes/Lobby/BP_LobbyGame.SpawnPlayer` _asbp_lobby_game self)
      (`KismetSystemLibrary.PrintString` "spawn 1"))
    (:`CastFailed`
      (`KismetSystemLibrary.PrintString` "NO FUNCO"))))

(fn `UserConstructionScript`)