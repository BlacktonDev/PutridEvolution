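; GS_BaseSetup is a game state that tracks lobby readiness and starts the match once everyone is ready.
; PlayerOnLobby adjusts the ReadyPlayers count and pushes it to each player's LobbyHUD widget.
; When the count matches PlayerArray, it creates a loading widget and server-travels to TopDownMap as a listen server.
; Other events recount ready BP_CarModel pawns or print player names for debugging, and both RepNotify functions are empty.
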(event `Player On Lobby`
  (params (IsReady :type Boolean))
  (bind _readyplayers (`self.ReadyPlayers`))
  (if IsReady
    (set `self.ReadyPlayers` (+ (`self.ReadyPlayers`) 1))
    (else
      (set `self.ReadyPlayers` (+ (`self.ReadyPlayers`) -1))))
  (for _array_element (`self.PlayerArray`)
    (`self.UpdatePlayersReadyUI` _readyplayers (`/Game/Pepongoc/Blueprints/GameModes/Lobby/LobbyHUD.UI_REF` (cast `/Game/Pepongoc/Blueprints/GameModes/Lobby/LobbyHUD` (`PlayerController.GetHUD` (`PlayerState.GetPlayerController` _array_element)) :!pure true)))
    (if (== _readyplayers (`KismetArrayLibrary.Array_Length` (`self.PlayerArray`)))
      (`|CreateWidget` "/Game/Pepongoc/Blueprints/UI/LoadMap/WB_Loading.WB_Loading_C")
      (`KismetSystemLibrary.ExecuteConsoleCommand` (`KismetStringLibrary.Concat_StrStr` "servertravel " "TopDownMap" "?listen") null))))

(event `self.ReceiveBeginPlay`
  (for _array_element (`self.PlayerArray`)
    (cast `/Game/Pepongoc/Blueprints/GameModes/PC_BaseSetup` (`PlayerState.GetPlayerController` _array_element))))

(event `UpdatePlayersReadyUI`
  (params (Players :type Integer) (`UI REF` :type "/Game/Pepongoc/Blueprints/UI/Lobby/WB_Lobby Object Reference"))
  (`/Game/Pepongoc/Blueprints/UI/Lobby/WB_Lobby.UpdatePlayersReady` `UI REF` Players))

(event `self.ReceiveTick`
  (params (DeltaSeconds :type "Float (single-precision)")))

(event `Update Player Num`
  (set `self.AllPlayerStates` (`self.PlayerArray`))
  (for _array_element _
    (`KismetSystemLibrary.PrintString` (`PlayerState.GetPlayerName` _array_element))))

(event `PlayersReady`
  (for _array_element (`self.AllPlayerStates`)
    (bind _asbp_car_model (cast `/Game/Pepongoc/Blueprints/BP_CarModel` (`Controller.K2_GetPawn` (`PlayerState.GetPlayerController` _array_element))))
    (if (`/Game/Pepongoc/Blueprints/BP_CarModel.IsPlayerReady` _asbp_car_model)
      (set `self.ReadyPlayers` (+ (`self.ReadyPlayers`) 1))))
  (`KismetSystemLibrary.PrintString` (`KismetStringLibrary.Conv_IntToString` (`self.ReadyPlayers`))))

(event `Server Player Ready`
  (for _array_element (`self.AllPlayerStates`)
    (bind _asbp_car_model (cast `/Game/Pepongoc/Blueprints/BP_CarModel` (`Controller.K2_GetPawn` (`PlayerState.GetPlayerController` _array_element))))
    (`KismetSystemLibrary.PrintString` (`PlayerState.GetPlayerName` _array_element))))

(fn `OnRep_AllPlayerStates`)

(fn `OnRep_ReadyPlayers`)

(fn `UserConstructionScript`)