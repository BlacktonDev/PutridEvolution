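; Lobby game mode that tracks connected players and can spawn them as cars.
; On BeginPlay it looks up the EIK session from the game instance's session ID to store the player limit.
; Login, controller swap and logout maintain the player list; login and logout also trigger a delayed GameState player-count update.
; A spawn function replaces a player's pawn with a possessed car at a random PlayerStart.
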(event `self.ReceiveBeginPlay`
  (bind _asbp_game_instance (cast `/Game/Pepongoc/Blueprints/UI/BP_GameInstance` (`GameplayStatics.GetGameInstance`)))
  (bind _foundresult (`EIK_FindSessionByID_AsyncFunction.FindEIKSessionByID` (`/Game/Pepongoc/Blueprints/UI/BP_GameInstance.SessionID` _asbp_game_instance))
    (:`OnSuccess`
      (set `self.Max Players` (`FindSessionsCallbackProxy.GetMaxPlayers` _foundresult)))))

(event `self.K2_PostLogin`
  (params (NewPlayer :type "PlayerController Object Reference"))
  (bind _aspc_base_setup (cast `/Game/Pepongoc/Blueprints/GameModes/PC_BaseSetup` NewPlayer))
  (`KismetArrayLibrary.Array_Add` (`self.All_Players`) _aspc_base_setup)
  (`self.Update Player Num` :!label _label))

(event `self.K2_OnSwapPlayerControllers`
  (params (OldPC :type "PlayerController Object Reference") (NewPC :type "PlayerController Object Reference"))
  (bind _aspc_base_setup (cast `/Game/Pepongoc/Blueprints/GameModes/PC_BaseSetup` NewPC))
  (`KismetArrayLibrary.Array_Add` (`self.All_Players`) _aspc_base_setup))

(event `Update Player Num`
  (`KismetSystemLibrary.Delay` 0.3)
  (bind _asgs_base_setup (cast `/Game/Pepongoc/Blueprints/GameModes/GS_BaseSetup` (`GameplayStatics.GetGameState`)))
  (`/Game/Pepongoc/Blueprints/GameModes/GS_BaseSetup.Update Player Num` _asgs_base_setup))

(event `self.K2_OnLogout`
  (params (ExitingController :type "Controller Object Reference"))
  (bind _aspc_base_setup (cast `/Game/Pepongoc/Blueprints/GameModes/PC_BaseSetup` ExitingController))
  (`KismetArrayLibrary.Array_RemoveItem` (`self.All_Players`) _aspc_base_setup)
  (goto _label))

(fn `Find Random PlayerStart`
  (returns (PlayerStart_Transform :type "Transform Structure (by ref)"))
  (bind _outactors (`GameplayStatics.GetAllActorsOfClass` "/Script/Engine.PlayerStart"))
  (return (`self.GetTransform` (`|GetArrayItem` _outactors (`KismetMathLibrary.RandomIntegerInRange` 0 (- (`KismetArrayLibrary.Array_Length` _outactors) 1))))))

(fn `SpawnPlayer`
  (params (PlayerController :type "PlayerController Object Reference"))
  (bind _returnvalue (`Controller.K2_GetPawn` PlayerController))
  (`/Engine/EditorBlueprintResources/StandardMacros.IsValid` _returnvalue
    (:`Is Valid`
      (`self.K2_DestroyActor` _returnvalue))
    (:`Is Not Valid`
      _))
  (bind _returnvalue_2 (`|SpawnActorFromClass` "/Game/Pepongoc/Blueprints/BP_CarModel.BP_CarModel_C" (`self.Find Random PlayerStart`) "AdjustIfPossibleButAlwaysSpawn" "MultiplyWithRoot" null null))
  (`Controller.Possess` PlayerController _returnvalue_2))

(fn `UserConstructionScript`)