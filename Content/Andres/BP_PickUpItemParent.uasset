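; Base actor for pickup items that hand themselves to whatever collects them on overlap.
; An overlapping actor implementing BI_PickUpItem, other than another pickup, receives the item class, icon and stack size by interface message, then the pickup destroys itself.
; PushPickUpItemAway launches the mesh along the camera's forward direction with a velocity-change impulse applied at an offset from the actor's location.
; GetPickUpItemData is a stub returning zero stack amounts.
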(event `self.ReceiveActorBeginOverlap`
  (params (OtherActor :type "Actor Object Reference"))
  (if (`KismetSystemLibrary.DoesImplementInterface` OtherActor "/Game/Andres/BI_PickUpItem.BI_PickUpItem_C")
    (if (not (`KismetMathLibrary.ClassIsChildOf` (`GameplayStatics.GetObjectClass` OtherActor) "BP_PickUpItemParent_C"))
      (message `/Game/Andres/BI_PickUpItem.PickUpItem` OtherActor (`self.ItemClass`) (`self.ItemIcon`) (`self.StackSize`))
      (`self.K2_DestroyActor`))))

(event `/Game/Andres/BI_PickUpItem.PushPickUpItemAway`
  (bind _returnvalue (`KismetMathLibrary.GetForwardVector` (`PlayerCameraManager.GetCameraRotation` (`GameplayStatics.GetPlayerCameraManager` 0))))
  (`PrimitiveComponent.AddVelocityChangeImpulseAtLocation` (`self.StaticMesh`) (* _returnvalue 250.0) (+ (`self.K2_GetActorLocation`) (+ _returnvalue (15.0 0.0 0.0))) "None"))

(fn `GetPickUpItemData`
  (returns (ItemClass :type "Actor Class Reference") (CurrentStackAmount :type Integer) (MaxStackAmount :type Integer))
  (return null 0 0))

(fn `UserConstructionScript`)